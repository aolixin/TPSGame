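; BP_WeaponInstance is a weapon instance Blueprint that plays the visual effects of firing.
; Its Fire event spawns two auto-destroying Niagara systems, a muzzle flash and a galaxy slash, both attached to the skeletal mesh at the Muzzle socket.
; The slash uses the socket's rotation, while the flash builds its rotation from that socket's up vector as the Y axis.
; The graph contains only effects, with no projectile or damage logic.
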(event Custom|Fire
  (bind _skeletalmesh (Variables|Default|GetSkeletalMesh))
  (bind _skeletalmesh_2 (Variables|Default|GetSkeletalMesh))
  (bind _returnvalue (Transformation|GetSocketTransform _skeletalmesh_2 "Muzzle" "RTS_Component"))
  (bind _returnvalue_2 (Transformation|GetSocketTransform _skeletalmesh "Muzzle" "RTS_Component"))
  (bind (_location _rotation) (Math|Transform|BreakTransform _returnvalue))
  (bind (_location_2 _rotation_2) (Math|Transform|BreakTransform _returnvalue_2))
  (Utilities|FlowControl|Sequence
    (:then_0
      (Niagara|SpawnSystemAttached "/Game/MuzzleFlash/Niagara/NS_MuzzleFlash.NS_MuzzleFlash" _skeletalmesh "None" _location_2 (Math|Rotator|MakeRotfromY (Math|Vector|GetUpVector _rotation_2)) "KeepRelativeOffset" true))
    (:then_1
      (Niagara|SpawnSystemAttached "/Game/MixedVFX/Particles/Slashes/NS_GalaxySlash.NS_GalaxySlash" _skeletalmesh_2 "None" _location _rotation "KeepRelativeOffset" true))))

(fn ConstructionScript)